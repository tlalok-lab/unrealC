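; Temperature actor Blueprint that reports temperature values as on-screen debug text.
; On BeginPlay it prints TemperatureCelsius and the result of GetTemperatureFahrenheit.
; The AbnormalTemperature event passes a fixed reading to OnTemperatureChecked, which prints its difference from zero via CalculateTemperatureDifference.
; The temperature helper functions are defined outside these graphs, and the construction script is empty.
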(event `self.ReceiveBeginPlay`
  ;[0 0.15 0.02729 0.5] Mostrar Variable en Viwport
  (`KismetSystemLibrary.PrintString` (`KismetStringLibrary.Concat_StrStr` "Temperatura:  " (`KismetStringLibrary.Conv_DoubleToString` (`self.TemperatureCelsius`))) true true (struct :`R` 0.619792 :`B` 0.157097 :`A` 1.0) 25.0)
  (`KismetSystemLibrary.PrintString` (`KismetStringLibrary.Concat_StrStr` (`KismetStringLibrary.Conv_DoubleToString` (`self.GetTemperatureFahrenheit`))) true true (struct :`R` 0.619792 :`B` 0.157097 :`A` 1.0) 25.0))

(event `AbnormalTemperature`
  (`self.OnTemperatureChecked` 28.0)
  (`KismetSystemLibrary.PrintString` "Hello" true true (struct :`R` 0.619792 :`B` 0.157097 :`A` 1.0) 25.0))

(event `self.OnTemperatureChecked`
  (params (CurrentTemperature :type "Float (single-precision)"))
  (bind _returnvalue (`self.CalculateTemperatureDifference` CurrentTemperature))
  (`KismetSystemLibrary.PrintString` (`KismetStringLibrary.Concat_StrStr` "Diferencia temperatura" (`KismetStringLibrary.Conv_DoubleToString` _returnvalue)) true true (struct :`R` 0.619792 :`B` 0.157097 :`A` 1.0) 25.0))

(fn `UserConstructionScript`)